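; Game-jam game mode that runs a timed collectable round on a grid of floor tiles.
; BeginPlay enables mouse and touch input, moves the BP_GGJ_Bicho pawn to a random tile, randomly spawns capped collectables and starts music and a death timer.
; Move_Made tracks the current tile, and RestartGrid resets tile states.
; RealEnding marks a win; it and timer-driven Death each show their own end widget, then reload the level after a delay.
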(event `Real Ending`
  (set `self.Win` true)
  (`GameplayStatics.SpawnSound2D` "/Game/Assets/Music/sfx_kittenllegada.sfx_kittenllegada" 1.0 1.0 0.0 null)
  (`self.GameOVer`))

(event `GameOVer`
  ;[1 1 1] Game Over Handler
  (bind _returnvalue (`|CreateWidget` "/Game/Blueprints/Widget/W_EndGame.W_EndGame_C"))
  (`UserWidget.AddToPlayerScreen` _returnvalue 0)
  (`KismetSystemLibrary.Delay` 5.0)
  (`GameplayStatics.OpenLevel` "Level"))

(event `Move_Made`
  (params (NewPosition :type "/Game/Blueprints/GameActors/BP_GGJ_Floor1 Object Reference"))
  (set `self.ActualPosition` NewPosition))

(event `self.ReceiveBeginPlay`
  (bind _returnvalue (`GameplayStatics.GetPlayerController` 0))
  ;[1 1 1] Initialize Controller and winning/lossing Conditions and create the main menu
  (set `PlayerController.bShowMouseCursor` true _returnvalue)
  (`KismetSystemLibrary.K2_SetTimerDelegate` (delegate `Death`) 55.0)
  ;[1 1 1] Enable the OnClicled event and remove Main menu from the screen
  (bind _outactors (`GameplayStatics.GetAllActorsOfClass` "/Game/Blueprints/GameActors/BP_GGJ_Bicho.BP_GGJ_Bicho_C"))
  (set `self.PlayerPawn` (`|GetArrayItem` _outactors))
  (set `PlayerController.bEnableClickEvents` true _returnvalue)
  (set `PlayerController.bEnableTouchEvents` true _returnvalue)
  ;[1 1 1] Put the Player Pawn on a validate initial position and spawn the items nessesaries to win the game
  (bind _outactors_2 (`GameplayStatics.GetAllActorsOfClass` "/Game/Blueprints/GameActors/BP_GGJ_Floor1.BP_GGJ_Floor1_C"))
  (set `self.Grid` _outactors_2)
  (bind _position (`self.Get Valid Position`))
  (set `/Game/Blueprints/GameActors/BP_GGJ_Floor1.State` 0 _position)
  (`/Game/Blueprints/GameActors/BP_GGJ_Floor1.Change Material` _position)
  (set `self.ActualPosition` _position)
  (`self.K2_SetActorLocation` (`self.PlayerPawn`) (+ (`self.K2_GetActorLocation` _position) (0.0 0.0 25.0)) false false)
  (`self.SpawnColectables`)
  (`GameplayStatics.SpawnSound2D` "/Game/Assets/Music/mus_juegoloop.mus_juegoloop" 1.0 1.0 0.0 null))

(event `Death`
  (bind _returnvalue (`|CreateWidget` "/Game/Blueprints/Widget/W_RealENd.W_RealENd_C"))
  (`UserWidget.AddToPlayerScreen` _returnvalue 0)
  (`KismetSystemLibrary.Delay` 5.0)
  (`GameplayStatics.OpenLevel` "Level"))

(fn `Calculate Chance`
  (returns (Good :type Boolean))
  (return (>= (* (`self.Posibilitys`) (`KismetMathLibrary.RandomFloatInRange` 0.0 1.0)) 0.8)))

(fn `Get Valid Position`
  (returns (Position :type "/Game/Blueprints/GameActors/BP_GGJ_Floor1 Object Reference"))
  (bind _grid (`self.Grid`))
  (bind _output (`|GetArrayItem` _grid (- (`KismetMathLibrary.RandomIntegerInRange` 1 (`KismetArrayLibrary.Array_Length` _grid)) 1)))
  (while (== (`/Game/Blueprints/GameActors/BP_GGJ_Floor1.State` _output) 0)
    _)
  (return _output))

(fn `RestartGrid`
  (for _array_element (`self.Grid`)
    (if (== (`/Game/Blueprints/GameActors/BP_GGJ_Floor1.State` _array_element) 1)
      (set `/Game/Blueprints/GameActors/BP_GGJ_Floor1.State` 0 _array_element)
      (`/Game/Blueprints/GameActors/BP_GGJ_Floor1.Change Material` _array_element))))

(fn `SpawnColectables`
  (bind _returnvalue (`self.GetTransform`))
  (for _array_element (`self.Grid`)
    (if (and (== (`/Game/Blueprints/GameActors/BP_GGJ_Floor1.State` _array_element) 0) (< (`self.ColectionablesOnWorld`) (`self.NeededObjects`)))
      (if (>= (`KismetMathLibrary.RandomIntegerInRange` 0 9) 6)
        (`|SpawnActorFromClass` "/Game/Blueprints/GameActors/BP_GGJ_Collectable.BP_GGJ_Collectable_C" (`KismetMathLibrary.MakeTransform` (`KismetMathLibrary.MakeVector` (.x (.location _returnvalue)) (.y (.location _returnvalue)) (+ (.z (.location _returnvalue)) 35.0)) (.rotation _returnvalue) (.scale _returnvalue)) "AlwaysSpawn" "OverrideRootScale" null null)
        (bind _result (`/Engine/EditorBlueprintResources/StandardMacros.IncrementInt` (`self.ColectionablesOnWorld`))
          (:`  `
            (set `self.ColectionablesOnWorld` _result)))))))

(fn `UserConstructionScript`)