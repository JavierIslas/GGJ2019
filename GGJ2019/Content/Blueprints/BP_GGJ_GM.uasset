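; Game mode for a game jam grid game where the player must collect a set number of objects before running out of turns.
; BeginPlay shows the main menu, then StartGame removes it and places the BP_GGJ_Bicho pawn on a random grid cell, intended to avoid State 2.
; Moves and pickups decrement counters that decide win or loss, leading to an end screen and delayed level restart.
; A helper provides a weighted random chance roll.
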(event `self.ReceiveBeginPlay`
  ;[1 1 1] Initialize Controller and winning/lossing Conditions
  (set `PlayerController.bShowMouseCursor` true (`GameplayStatics.GetPlayerController` 0))
  (set `self.TurnsRemaining` 75)
  (set `self.NeededObjects` 5)
  (bind _returnvalue (`|CreateWidget` "/Game/Blueprints/Widget/W_MainMenu.W_MainMenu_C" (`GameplayStatics.GetPlayerController` 0)))
  (`UserWidget.AddToPlayerScreen` _returnvalue 0)
  (set `self.Widget` _returnvalue))

(event `StartGame`
  (bind _returnvalue (`GameplayStatics.GetPlayerController` 0))
  (`Widget.RemoveFromParent` (`self.Widget`))
  (bind _outactors (`GameplayStatics.GetAllActorsOfClass` "/Game/Blueprints/GameActors/BP_GGJ_Bicho.BP_GGJ_Bicho_C"))
  (set `self.PlayerPawn` (`|GetArrayItem` _outactors))
  (set `PlayerController.bEnableClickEvents` true _returnvalue)
  (set `PlayerController.bEnableTouchEvents` true _returnvalue)
  (bind _position (`self.Get Valid Position`))
  (`self.K2_SetActorLocation` (`self.PlayerPawn`) (`self.K2_GetActorLocation` _position) false false))

(event `Move_Made`
  (params (NewPosition :type "/Game/Blueprints/GameActors/BP_GGJ_Floor Object Reference"))
  ;[1 1 1] Handle lossing Condition
  (bind _result (`/Engine/EditorBlueprintResources/StandardMacros.DecrementInt` (`self.TurnsRemaining`))
    (:`  `
      (bind _output_get (set `self.TurnsRemaining` _result))
      (if (<= _output_get 0)
        (set `self.Win` false)
        (`self.GameOVer`)
        (else
          (set `self.ActualPosition` NewPosition))))))

(event `GameOVer`
  ;[1 1 1] Game Over Handler
  (bind _returnvalue (`|CreateWidget` "/Game/Blueprints/Widget/W_EndGame.W_EndGame_C"))
  (`UserWidget.AddToPlayerScreen` _returnvalue 0)
  (`KismetSystemLibrary.Delay` 5.0)
  (`KismetSystemLibrary.ExecuteConsoleCommand` "RestartLevel" null))

(event `PickUpObject`
  ;[1 1 1] Handle winning condition
  (bind _result (`/Engine/EditorBlueprintResources/StandardMacros.DecrementInt` (`self.NeededObjects`))
    (:`  `
      (if (<= _result 0)
        (set `self.Win` true)
        (`self.GameOVer`)))))

(fn `Calculate Chance`
  (returns (Good :type Boolean))
  (return (>= (* (`self.Posibilitys`) (`KismetMathLibrary.RandomFloatInRange` 0.0 1.0)) 0.8)))

(fn `Get Valid Position`
  (returns (Position :type "/Game/Blueprints/GameActors/BP_GGJ_Floor Object Reference"))
  (bind _grid (`self.Grid`))
  (bind _output (`|GetArrayItem` _grid (`KismetMathLibrary.RandomIntegerInRange` 0 (- (`KismetArrayLibrary.Array_Length` _grid) 1))))
  (while (== (`/Game/Blueprints/GameActors/BP_GGJ_Floor.State` _output) 2)
    _)
  (return _output))

(fn `UserConstructionScript`)