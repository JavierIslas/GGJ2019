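; Clickable or touchable floor tile for a grid movement puzzle, where the player steps only onto free neighboring tiles.
; A valid tap moves the pawn here, marks the tile red and reports the move to GM; with no current position, any free tile is valid.
; Tapping a non-free tile ends the game if no neighbor of the current position is free.
; The construction script colors each tile by its State.
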(event `self.ReceiveBeginPlay`
  (bind (_asbp_ggj_gm _bsuccess) (cast `/Game/Blueprints/BP_GGJ_GM` (`GameplayStatics.GetGameMode`) :!pure true))
  (if _bsuccess
    (set `self.GM` _asbp_ggj_gm)))

(event `self.ReceiveActorOnInputTouchEnter`
  (params (FingerIndex :type "ETouchIndex Enum" :default "Touch1"))
  (bind _gm (`self.GM`))
  (bind _actualposition (`/Game/Blueprints/BP_GGJ_GM.ActualPosition` _gm))
  ;[1 1 1] Move Player to new location
  (if (== (`self.State`) 0) :!label _label
    (bind _binarray (`self.CheckPosition` _actualposition))
    (if _binarray
      (`self.K2_SetActorLocation` (`/Game/Blueprints/BP_GGJ_GM.PlayerPawn` _gm) (`self.K2_GetActorLocation`) false false)
      ;;[1 1 1] Change floor state
      (set `self.State` 1)
      (`PrimitiveComponent.SetMaterial` (`self.Body`) 0 "/Game/Assets/ProtAssetes/M_Color_Red_Inst.M_Color_Red_Inst")
      (`/Game/Blueprints/BP_GGJ_GM.Move_Made` _gm self))
    (else
      ;[1 1 1] Checks if there's no valide movement
      (bind _unwinnable (`self.CheckSoftLock` _actualposition))
      (if _unwinnable
        (`/Game/Blueprints/BP_GGJ_GM.GameOVer` _gm)))))

(event `self.ReceiveActorOnClicked`
  (params (ButtonPressed :type "Key Structure"))
  ;[1 1 1] Move Player to new location
  (goto _label))

(fn `CheckPosition`
  (params (LastPosition :type "/Game/Blueprints/BP_GGJ_Floor Object Reference"))
  (returns (bInArray :type Boolean))
  (if (!= LastPosition null)
    (for _array_element (`/Game/Blueprints/BP_GGJ_Floor.Neighbors` LastPosition)
      (if (== _array_element self)
        (return true)))
    (return false)
    (else
      (return true))))

(fn `CheckSoftLock`
  (params (Position :type "/Game/Blueprints/BP_GGJ_Floor Object Reference"))
  (returns (Unwinnable :type Boolean))
  (for _array_element (`/Game/Blueprints/BP_GGJ_Floor.Neighbors` Position)
    (if (== (`/Game/Blueprints/BP_GGJ_Floor.State` _array_element) 0)
      (return false)))
  (return true))

(fn `UserConstructionScript`
  (bind _body (`self.Body`))
  (switch `int` (`self.State`)
    (:`0`
      (`PrimitiveComponent.SetMaterial` _body 0 "/Game/Assets/ProtAssetes/M_Color_Green_Inst.M_Color_Green_Inst"))
    (:`1`
      (`PrimitiveComponent.SetMaterial` _body 0 "/Game/Assets/ProtAssetes/M_Color_Red_Inst.M_Color_Red_Inst"))
    (:`2`
      (`PrimitiveComponent.SetMaterial` _body 0 "/Game/Assets/ProtAssetes/M_Color_Blue_Inst.M_Color_Blue_Inst"))))