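; BP_GGJ_Bicho is an animated creature actor using Gata animations that starts in a looping idle with zeroed rotation.
; Custom events turn it 45 degrees in yaw per call or glide it to a given relative location over a fixed time.
; PlayJump plays one of two randomly chosen jump animations, then returns to idle after a fixed delay.
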(event `self.ReceiveBeginPlay`
  (`SkeletalMeshComponent.PlayAnimation` (`self.Body`) "/Game/Assets/Meshes/Animations/gata_01_Idle.gata_01_Idle" true)
  (`self.K2_SetActorRotation` (struct)))

(event `RotateActor`
  (bind (_returnvalue_roll _returnvalue_pitch _returnvalue_yaw) (`KismetMathLibrary.BreakRotator` (`self.K2_GetActorRotation`)))
  (`self.K2_SetActorRotation` (`KismetMathLibrary.MakeRotator` _returnvalue_roll _returnvalue_pitch (+ _returnvalue_yaw 45.0))))

(event `Move`
  (params (Location :type "Vector Structure"))
  (`KismetSystemLibrary.MoveComponentTo` null Location (struct) false false 2.5))

(event `Play Jump`
  (bind _body (`self.Body`))
  (switch `int` (`KismetMathLibrary.RandomIntegerInRange` 1 2)
    (:`Default`
      (`SkeletalMeshComponent.PlayAnimation` _body "/Game/Assets/Meshes/Animations/gata_01_Jump1.gata_01_Jump1" false :!label _label))
    (:`1`
      (goto _label))
    (:`2`
      (`SkeletalMeshComponent.PlayAnimation` _body "/Game/Assets/Meshes/Animations/gata_01_Jump2.gata_01_Jump2" false)))
  (`KismetSystemLibrary.Delay` 3.0)
  (`SkeletalMeshComponent.PlayAnimation` (`self.Body`) "/Game/Assets/Meshes/Animations/gata_01_Idle.gata_01_Idle" true))

(fn `UserConstructionScript`)