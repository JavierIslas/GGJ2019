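; BP_GGJ_Floor is a grid floor tile that the player taps or clicks to move the pawn onto it.
; A free tile accepts a move if it neighbors the current position or none exists, then turns red and notifies the game mode.
; Tapping a used or blocked tile triggers game over when no free neighbor remains.
; Construction applies state materials and random obstacle meshes for blocked tiles, and BeginPlay asks the game mode to spawn collectables.
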(event `self.ReceiveBeginPlay`
  (bind (_asbp_ggj_gm _bsuccess) (cast `/Game/Blueprints/BP_GGJ_GM` (`GameplayStatics.GetGameMode`) :!pure true))
  (if _bsuccess
    (bind _output_get (set `self.GM` _asbp_ggj_gm))
    (`/Game/Blueprints/BP_GGJ_GM.SpawnColectables` _output_get)))

(event `self.ReceiveActorOnInputTouchEnter`
  (params (FingerIndex :type "ETouchIndex Enum" :default "Touch1"))
  (bind _gm (`self.GM`))
  (bind _actualposition (`/Game/Blueprints/BP_GGJ_GM.ActualPosition` _gm))
  ;[1 1 1] Move Player to new location
  (if (== (`self.State`) 0) :!label _label
    (bind _binarray (`self.CheckPosition` _actualposition))
    (if _binarray
      (`/Game/Blueprints/GameActors/BP_GGJ_Bicho.Move` (`/Game/Blueprints/BP_GGJ_GM.PlayerPawn` _gm) (`self.K2_GetActorLocation`))
      ;;[1 1 1] Change floor state
      (set `self.State` 1)
      (`self.Change Material`)
      (`/Game/Blueprints/BP_GGJ_GM.Move_Made` _gm self))
    (else
      ;[1 1 1] Checks if there's no valide movement
      (bind _unwinnable (`self.CheckSoftLock` _actualposition))
      (if _unwinnable
        (`/Game/Blueprints/BP_GGJ_GM.GameOVer` _gm)))))

(event `self.ReceiveActorOnClicked`
  (params (ButtonPressed :type "Key Structure"))
  ;[1 1 1] Move Player to new location
  (goto _label))

(fn `Change Material`
  (bind _body (`self.Body`))
  (switch `int` (`self.State`)
    (:`0`
      (`PrimitiveComponent.SetMaterial` _body 0 "/Game/Assets/Meshes/Statics/pasto_textura_Mat.pasto_textura_Mat"))
    (:`1`
      (`PrimitiveComponent.SetMaterial` _body 0 "/Game/Assets/Materials/M_Color_Red_Inst.M_Color_Red_Inst"))
    (:`2`
      (`PrimitiveComponent.SetMaterial` _body 0 null))))

(fn `Change Meshes`
  (bind _block (`self.Block`))
  (bind _meshes (`self.Meshes`))
  (if (== (`self.State`) 2)
    (`SceneComponent.SetVisibility` _block true false)
    (`StaticMeshComponent.SetStaticMesh` _block (`|GetArrayItem` _meshes (`KismetMathLibrary.RandomIntegerInRange` 0 (- (`KismetArrayLibrary.Array_Length` _meshes) 1))))))

(fn `CheckPosition`
  (params (LastPosition :type "/Game/Blueprints/GameActors/BP_GGJ_Floor Object Reference"))
  (returns (bInArray :type Boolean))
  (if (!= LastPosition null)
    (for _array_element (`/Game/Blueprints/GameActors/BP_GGJ_Floor.Neighbors` LastPosition)
      (if (== _array_element self)
        (return true)))
    (return false)
    (else
      (return true))))

(fn `CheckSoftLock`
  (params (Position :type "/Game/Blueprints/GameActors/BP_GGJ_Floor Object Reference"))
  (returns (Unwinnable :type Boolean))
  (for _array_element (`/Game/Blueprints/GameActors/BP_GGJ_Floor.Neighbors` Position)
    (if (== (`/Game/Blueprints/GameActors/BP_GGJ_Floor.State` _array_element) 0)
      (return false)))
  (return true))

(fn `SelectState`
  (returns (State :type Integer))
  (if (>= (`KismetMathLibrary.RandomIntegerInRange` 0 100) 80)
    (return 2)
    (else
      (return 0))))

(fn `UserConstructionScript`
  (`self.Change Meshes`)
  (`self.Change Material`))