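; BP_GGJ_Collectable is a pickup actor that a BP_GGJ_Bicho collects by touching it.
; The construction script gives the Body a random mesh from the Meshes array, and Tick spins the actor with a small fixed rotation each frame.
; When a Bicho overlaps the Sphere, it plays a pickup sound, calls PickUpObject on the BP_GGJ_GM game mode and destroys itself.
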(event `self.ReceiveBeginPlay`
  (`ActorComponent.SetComponentTickInterval` (`self.Body`) 1.0))

(event `self.ReceiveTick`
  (params (DeltaSeconds :type "Float (single-precision)"))
  ;[1 1 1] Animation
  (`self.K2_AddActorLocalRotation` (struct :`Pitch` 1.0 :`Yaw` 3.0 :`Roll` 0.5)))

(event `self.Sphere.OnComponentBeginOverlap`
  (params (OverlappedComponent :type "PrimitiveComponent Object Reference") (OtherActor :type "Actor Object Reference") (OtherComp :type "PrimitiveComponent Object Reference") (OtherBodyIndex :type Integer) (bFromSweep :type Boolean) (SweepResult :type "HitResult Structure (by ref)"))
  (bind (_asbp_ggj_gm _bsuccess) (cast `/Game/Blueprints/BP_GGJ_GM` (`GameplayStatics.GetGameMode`) :!pure true))
  ;[1 1 1] Collition Handle
  (if (`.bSuccess` (cast `/Game/Blueprints/GameActors/BP_GGJ_Bicho` OtherActor :!pure true))
    (`GameplayStatics.PlaySoundAtLocation` "/Game/Assets/Music/sfx_getcomida_Cue.sfx_getcomida_Cue" (`self.K2_GetActorLocation`) (struct) 1.0 1.0 0.0 null null null)
    (if _bsuccess
      (`/Game/Blueprints/BP_GGJ_GM.PickUpObject` _asbp_ggj_gm)
      (`self.K2_DestroyActor`))))

(fn `UserConstructionScript`
  (bind _meshes (`self.Meshes`))
  (`StaticMeshComponent.SetStaticMesh` (`self.Body`) (`|GetArrayItem` _meshes (`KismetMathLibrary.RandomIntegerInRange` 0 (- (`KismetArrayLibrary.Array_Length` _meshes) 1)))))